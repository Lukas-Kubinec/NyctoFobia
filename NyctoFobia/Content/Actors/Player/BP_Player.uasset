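; Player character for a sanity horror game, handling the intro, Escape pause via time dilation, and game-over restart.
; FireLight overlaps pause sanity loss and reset the meter held in the UI widget, while Monster contact maxes insanity.
; Tick drives delayed random spook sounds, insanity-smoothed fog and, while insanity is above zero, timed monster spawns around the player.
; Game-over and win flags live in BP_GameInstance; custom C++ helpers pick random sounds and locations.
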(event `GameIntro`
  ;[0.02418 0.15 0.1198 0.5] Game Intro
  (`self.Crouch`) ; Makes the character crouch
  (`PlayerCameraManager.StartCameraFade` :`self` (`GameplayStatics.GetPlayerCameraManager` 0) :`FromAlpha` 1.0 :`Duration` 4.0 :`bShouldFadeAudio` true) ; Game fade transition
  (`KismetSystemLibrary.Delay` 3.0)
  (`GameplayStatics.PlaySound2D` "/Game/Dialogue/RAW/dialogue_01.dialogue_01" 1.0 1.0 0.0 null null) ; Plays the first dialog after delay
  (`KismetSystemLibrary.Delay` 4.0)
  (`self.UnCrouch`) ; Uncrouches the player
  (set `self.canMove` true) ; Enables the character movement
  (set `self.IsAwake` true)
  (bind _returnvalue (`|CreateWidget` "/Game/Actors/Widgets/InGameUI.InGameUI_C"))
  (`UserWidget.AddToViewport` _returnvalue 0) ; Adds the game UI once the intro is over
  (set `self.GameUI_Widget` _returnvalue)
  (bind _returnvalue_2 (`|CreateWidget` "/Game/Actors/Widgets/PauseScreen.PauseScreen_C")) ; Creates Pause screen that is shown/hidden when ESC is pressed
  (set `self.PauseUI` _returnvalue_2))

(event `self.ReceiveBeginPlay`
  ;[1 0.02233 0] EVENT FUNCTIONS
  ;; Event Begin Play
  (bind _asbp_game_instance (cast `/Game/Actors/BP_GameInstance` (`GameplayStatics.GetGameInstance`)))
  (set `/Game/Actors/BP_GameInstance.IsGameWon` false _asbp_game_instance)
  (set `/Game/Actors/BP_GameInstance.IsGameOver` false _asbp_game_instance)
  (set `self.canMove` false) ; Disables Player movement
  (set `self.IsAwake` false)
  (`self.DisableLockCursor`)
  (`self.GameIntro`))

(event `EnterCollisionFireLamp`
  (params (OtherActor :type "Actor Object Reference"))
  ;[0.3 0.2135 0.6406] COLLISIONS
  ;; Check for Enter Collision with the fire lamp light
  (`KismetSystemLibrary.DelayUntilNextTick`)
  (bind _asbp_game_instance (cast `/Game/Actors/BP_GameInstance` (`GameplayStatics.GetGameInstance`)))
  (if (and (not (`/Game/Actors/BP_GameInstance.IsGameOver` _asbp_game_instance)) (`self.ActorHasTag` OtherActor "FireLight") (`self.canMove`))
    (set `/Game/Actors/Widgets/InGameUI.IsPlayerNearLight` true (`self.GameUI_Widget`)) ; Disables the decreament of sanity
    (`GameplayStatics.PlaySound2D` (`RandomSoundEffectComponent.ChooseRandomSoundEffect` (`|MakeArray` "/Game/Dialogue/sound_relief_01_Cue.sound_relief_01_Cue" "/Game/Dialogue/sound_relief_02_Cue.sound_relief_02_Cue" "/Game/Dialogue/sound_relief_03_Cue.sound_relief_03_Cue" "/Game/Dialogue/sound_relief_04_Cue.sound_relief_04_Cue" :!type "SoundBase Object Reference")) 1.0 1.0 0.0 null null) ; Plays random voice line
    (`self.ResetSanityMeter`) ; Resets the sanity values
  ))

(event `self.ReceiveTick`
  (params (DeltaSeconds :type "Float (single-precision)"))
  ;[1 0.02233 0] EVENT FUNCTIONS
  ;; Event Tick
  (`self.CheckIsGameOver` null)
  (`self.PlayRandomSpookSound`)
  (`self.HandleFog`)
  (`self.SpawnMonster`))

(event `CheckIsGameOver`
  (params (OtherActor :type "Actor Object Reference"))
  ; Check if the Game is Over
  (bind _asbp_game_instance (cast `/Game/Actors/BP_GameInstance` (`GameplayStatics.GetGameInstance`)))
  (if (and (`/Game/Actors/BP_GameInstance.IsGameOver` _asbp_game_instance) (not (`/Game/Actors/BP_GameInstance.IsGameWon` _asbp_game_instance)))
    (set `self.canMove` false)
    (`self.Crouch`)
    (if (`Widget.IsRendered` (`self.GameUI_Widget`))
      (`WidgetLayoutLibrary.RemoveAllWidgets`)
      (else
        (`KismetSystemLibrary.DelayUntilNextTick`)
        (`/Engine/EditorBlueprintResources/StandardMacros.DoOnce` false
          (:`Completed`
            (bind _returnvalue (`|CreateWidget` "/Game/Actors/Widgets/InGameOverUI.InGameOverUI_C"))
            (bind _output_get (set `self.GameOverUI_Widget` _returnvalue))
            (if (not (`Widget.IsRendered` (`self.GameOverUI_Widget`)))
              (`UserWidget.AddToViewport` _output_get 1)
              (`ActorComponent.K2_DestroyComponent` (`self.Lantern`))
              (`self.RestartLevel` null))))))))

(event `LeaveCollisionFireLamp`
  (params (OtherActor :type "Actor Object Reference"))
  ;[0.3 0.2135 0.6406] COLLISIONS
  ;; Check for Leave Collision with the fire lamp light
  (if (`self.ActorHasTag` OtherActor "FireLight")
    (set `/Game/Actors/Widgets/InGameUI.IsPlayerNearLight` false (`self.GameUI_Widget`)) ; Starts the decreament of sanity meter
  ))

(event `self.ReceiveActorEndOverlap`
  (params (OtherActor :type "Actor Object Reference"))
  ;[1 0.02233 0] EVENT FUNCTIONS
  ;; Leave Collision check
  (`self.LeaveCollisionFireLamp` OtherActor))

(event `RestartLevel`
  (params (OtherActor :type "Actor Object Reference"))
  ; Restarts level
  (`KismetSystemLibrary.Delay` 3.0)
  (bind _returnvalue (`GameplayStatics.GetCurrentLevelName` true))
  (`LevelStreamingDynamic.LoadLevelInstance` _returnvalue (0.0 0.0 0.0) (struct) "" null) ; Restarts the current level
  (`GameplayStatics.OpenLevel` (`KismetStringLibrary.Conv_StringToName` _returnvalue)))

(event `self.ReceiveActorBeginOverlap`
  (params (OtherActor :type "Actor Object Reference"))
  ;[1 0.02233 0] EVENT FUNCTIONS
  ;; Enter Collision check
  (`self.EnterCollisionFireLamp` OtherActor)
  (`self.EnterCollisionMonster` OtherActor))

(event `EnterCollisionMonster`
  (params (OtherActor :type "Actor Object Reference"))
  ;[0.3 0.2135 0.6406] COLLISIONS
  ;; Check for Enter Collision with the Monster
  (if (`self.ActorHasTag` OtherActor "Monster")
    (set `/Game/Actors/Widgets/InGameUI.Insanity_Value` 1.0 (`self.GameUI_Widget`)) ; Makes the player insane - game over
  ))

(event `Key|Escape`
  (params (Key :type "Key Structure"))
  ;[1 0.02233 0] EVENT FUNCTIONS
  ;; Pause Menu
  (:`Pressed`
    (bind _asbp_game_instance (cast `/Game/Actors/BP_GameInstance` (`GameplayStatics.GetGameInstance`)))
    (if (`/Game/Actors/BP_GameInstance.IsGameOver` _asbp_game_instance)
      _
      (elif (`self.IsAwake`)
        (if (`self.IsGamePaused`)
          (`GameplayStatics.SetGlobalTimeDilation` 1.0) ; Unpauses world
          (set `self.IsGamePaused` false)
          (set `self.canMove` true) ; Enables movement
          (`Widget.RemoveFromParent` (`self.PauseUI`)) ; Removes pause screen
          (else
            (`GameplayStatics.SetGlobalTimeDilation` 0.0) ; Pauses the world
            (set `self.IsGamePaused` true)
            (set `self.canMove` false) ; Disables movement
            (`UserWidget.AddToPlayerScreen` (`self.PauseUI`) 0) ; Adds pause screen
          ))))))

(event `SpawnMonster`
  ; Spawn Monster when insanity is over 0
  (`/Engine/EditorBlueprintResources/StandardMacros.CompareFloat` (`/Game/Actors/Widgets/InGameUI.Insanity_Value` (`self.GameUI_Widget`)) ; Checks if insanity is above zero
    (:`>`
      (`/Engine/EditorBlueprintResources/StandardMacros.DoOnce` false :!label _label ; Makes a new reaper spawn every 3 seconds\nThis check is reset every time a reaper is spawned
        (:`Completed`
          (`KismetSystemLibrary.Delay` 3.0)
          (bind _returnvalue (`RandomLocationAroundActor.GetRandomLocationAroundActor` (`self.K2_GetActorLocation`) 1200.0 50.0)) ; Custom C++ function - \nGenerates random location
          (`|SpawnActorFromClass` "/Game/Actors/Monster/BP_Monster.BP_Monster_C" (`KismetMathLibrary.MakeTransform` _returnvalue) "AdjustIfPossibleButAlwaysSpawn" "MultiplyWithRoot" null null) ; Spawns new Monster at random location
          (goto _label :!via `Reset`))))))

(event `ResetSanityMeter`
  ;[1 0.02233 0] EVENT FUNCTIONS
  ;; Resets the Sanity level
  (`/Game/Actors/Widgets/InGameUI.Set_ResetSanity` (`self.GameUI_Widget`)) ; Resets the sanity values
)

(event `PlayRandomSpookSound`
  ; Plays random spooky sounds around the player
  (`KismetSystemLibrary.Delay` (`KismetMathLibrary.RandomFloatInRange` 5.0 10.0))
  (bind _returnvalue (`RandomLocationAroundActor.GetRandomLocationAroundActor` (`self.K2_GetActorLocation`) 500.0 20.0)) ; Custom C++ function - \nGets location around the player \nso it can be used to spawn a new\nsound effect
  (`GameplayStatics.PlaySoundAtLocation` (`RandomSoundEffectComponent.ChooseRandomSoundEffect` (`|MakeArray` "/Game/Sounds/spook_01_Cue.spook_01_Cue" "/Game/Sounds/spook_02_Cue.spook_02_Cue" "/Game/Sounds/spook_03_Cue.spook_03_Cue" "/Game/Sounds/spook_04_Cue.spook_04_Cue" "/Game/Sounds/spook_05_Cue.spook_05_Cue" "/Game/Sounds/spook_06_Cue.spook_06_Cue" "/Game/Sounds/spook_07_Cue.spook_07_Cue" "/Game/Sounds/spook_08_Cue.spook_08_Cue" "/Game/Sounds/spook_09_Cue.spook_09_Cue" :!type "SoundBase Object Reference")) _returnvalue (struct) 1.0 1.0 0.0 "/Game/Sounds/attentuation_long_distance.attentuation_long_distance" null null null) ; Plays the sound effect around the player
)

(event `DisableLockCursor`
  ; Disable and Lock the cursor
  (set `PlayerController.bShowMouseCursor` false (`GameplayStatics.GetPlayerController` 0))
  (`WidgetBlueprintLibrary.SetHardwareCursor` "None") ; Hides the cursor
  (`WidgetBlueprintLibrary.SetFocusToGameViewport`) ; Focus on the game window
)

(event `HandleFog`
  (bind _playerfogcomponent (`self.PlayerFogComponent`))
  (bind _returnvalue (+ (`KismetMathLibrary.WeightedMovingAverage_Float` (* (`/Game/Actors/Widgets/InGameUI.Insanity_Value` (`self.GameUI_Widget`)) 3.0) (`LocalFogVolumeComponent.RadialFogExtinction` (`self.PlayerFogComponent`)) 0.1) 0.05))
  ; Manages Fog using the Insanity value
  (`LocalFogVolumeComponent.SetHeightFogExtinction` _playerfogcomponent _returnvalue) ; Sets the fog using the insanity level
  (`LocalFogVolumeComponent.SetRadialFogExtinction` _playerfogcomponent _returnvalue))

(fn `UserConstructionScript`)