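; Monster actor (a reaper) that chases the player and emits a positional sound until the game is over.
; Tick drives two custom events, AI and PlayMonsterSound, which both check IsGameOver on BP_GameInstance.
; AI rotates the actor toward the player and uses MoveComponentTo to move MeshCollider to the player's location, stopping it at game over.
; The sound uses long-distance attenuation and a DoOnce gate, with its volume zeroed at game over.
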(event `PlayMonsterSound`
  (params (DeltaSeconds :type "Float (single-precision)"))
  ; Sound effect
  (bind _asbp_game_instance (cast `/Game/Actors/BP_GameInstance` (`GameplayStatics.GetGameInstance`)))
  (if (`/Game/Actors/BP_GameInstance.IsGameOver` _asbp_game_instance)
    (set `self.MonsterSoundVolume` 0.0) ; Disables the monster sound \nif the game is over
    (else
      (`/Engine/EditorBlueprintResources/StandardMacros.DoOnce` false ; Starts to play the sound just once
        (:`Completed`
          _))))
  (`GameplayStatics.PlaySoundAtLocation` "/Game/Sounds/soundcue_monster.soundcue_monster" (`self.K2_GetActorLocation`) (struct) (`self.MonsterSoundVolume`) 1.0 0.0 "/Game/Sounds/attentuation_long_distance.attentuation_long_distance" null null null) ; Gives the reaper sound
)

(event `self.ReceiveBeginPlay`
  ; Event Begin Play
)

(event `self.ReceiveTick`
  (params (DeltaSeconds :type "Float (single-precision)"))
  ; Event Tick
  (`self.AI` 0.0)
  (`self.PlayMonsterSound` 0.0))

(event `AI`
  (params (DeltaSeconds :type "Float (single-precision)"))
  ; AI - Follow & Rotate towards Player
  (bind _asbp_game_instance (cast `/Game/Actors/BP_GameInstance` (`GameplayStatics.GetGameInstance`)))
  (if (`/Game/Actors/BP_GameInstance.IsGameOver` _asbp_game_instance)
    (goto _label :!via `Stop`)
    (else
      (`self.K2_SetActorRotation` (`KismetMathLibrary.Conv_VectorToRotator` (`KismetMathLibrary.Normal` (- (`self.K2_GetActorLocation` (`GameplayStatics.GetPlayerPawn` 0)) (`self.K2_GetActorLocation`))))) ; Rotates towards the player
      (`KismetSystemLibrary.MoveComponentTo` (`self.MeshCollider`) (`self.K2_GetActorLocation` (`GameplayStatics.GetPlayerPawn` 0)) (struct) false false 1.5 :!label _label) ; Chases the player
    )))

(fn `UserConstructionScript`)